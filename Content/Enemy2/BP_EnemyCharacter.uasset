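; Enemy character Blueprint that takes damage and passes perceived pawns to its AI blackboard as targets.
; AnyDamage subtracts the damage from CurrentHealth and prints debug messages, with no clamp or death check.
; Its AIPerception component writes any updated pawn to the TargetActor key, without checking whether it was sensed or lost.
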(event OnTargetPerceptionUpdated(AIPerception)
  (params (Actor :type Actor%20Object%20Reference) (Stimulus :type AI%20Stimulus%20Structure))
  (bind _as폰 (Utilities|Casting|CastToPawn Actor))
  (AI|Components|Blackboard|SetValueasObject (AI|GetBlackboard 0) (Variables|Default|GetTarget%20Actor) _as폰))

(event Game|Damage|EventAnyDamage
  (params (Damage :type Float%20%28single-precision%29) (DamageType :type Damage%20Type%20Object%20Reference) (InstigatedBy :type Controller%20Object%20Reference) (DamageCauser :type Actor%20Object%20Reference))
  (Utilities|FlowControl|Sequence
    (:then_0
      (Development|PrintString "데미지 입는중")
      (bind _output_get (Variables|Default|SetCurrent%20Health (- (Variables|Default|GetCurrent%20Health) Damage)))
      (Development|PrintString (Utilities|String|ToString(Float) _output_get)))))

(fn ConstructionScript)