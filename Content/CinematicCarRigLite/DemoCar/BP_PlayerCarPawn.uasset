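; Player car pawn that drives on FloatingPawnMovement with drifting steering and a boost gauge.
; Move input sets a throttle-scaled yaw target and feeds a drift helper that blends heading with velocity and counters sideways slip using lateral friction.
; Each Tick, the 자동차구동 graph eases controller yaw toward that target and handles boost.
; Held boost raises max speed while draining the gauge, which starts empty and regenerates otherwise.
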(event Input|EnhancedActionEvents|EnhancedInputActionIA_MoveMent
  (params (ActionValue :type Vector%202D%20Structure) (ElapsedSeconds :type Float%20%28double-precision%29) (TriggeredSeconds :type Float%20%28double-precision%29) (InputAction :type Input%20Action%20Object%20Reference :default "/Game/CinematicCarRigLite/DemoCar/IA_MoveMent.IA_MoveMent"))
  (bind _returnvalue (Pawn|GetControlRotation :!class /Script/Engine.Pawn))
  (bind _yaw (Math|Rotator|BreakRotator _returnvalue))
  (bind _returnvalue_2 (Math|Rotator|MakeRotator 0.0 0.0 _yaw))
  (bind _returnvalue_3 (Math|Vector|GetRightVector _returnvalue_2))
  (:Triggered
    (Variables|Default|SetYawSpeedTarget (* (* (.x ActionValue) (.y ActionValue)) (Variables|Default|GetTurnRate)) :!label _label)
    (Pawn|Input|AddMovementInput (.SlipDirection (Utilities|드리프트설정 (Math|Vector|GetForwardVector _returnvalue_2) _returnvalue_3 (Variables|Default|GetDriftAlpha) (Variables|Default|GetLateralFriction) (stale EventTick DeltaSeconds))) (.y ActionValue) false)
    (Pawn|Input|AddMovementInput _returnvalue_3 (* (.LateralScale (Utilities|드리프트설정 (Math|Vector|GetForwardVector _returnvalue_2) _returnvalue_3 (Variables|Default|GetDriftAlpha) (Variables|Default|GetLateralFriction) (stale EventTick DeltaSeconds))) -1.0) false))
  (:Ongoing
    (goto _label)))

(event Input|EnhancedActionEvents|EnhancedInputActionIA_CarBoost
  (params (ActionValue :type Boolean) (ElapsedSeconds :type Float%20%28double-precision%29) (TriggeredSeconds :type Float%20%28double-precision%29) (InputAction :type Input%20Action%20Object%20Reference :default "/Game/CinematicCarRigLite/DemoCar/IA_CarBoost.IA_CarBoost"))
  (:Started
    (Variables|Default|SetbBoostHeld true))
  (:Completed
    (Variables|Default|SetbBoostHeld false)))

(event EventBeginPlay
  (Variables|Default|SetBoostGauge 0.0))

(event EventTick
  (params (DeltaSeconds :type Float%20%28single-precision%29))
  (Utilities|자동차구동 DeltaSeconds))

(fn ConstructionScript)