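; Flamethrower weapon Blueprint that switches a flame effect and looping audio on and off with the fire input.
; IA_Fire Started and Completed call StartFire and StopFire, which use an Active flag to ignore redundant calls.
; These functions play or stop AudioFlameLoop, activate or deactivate NSFlame, and print debug strings.
; The graphs contain no damage, hit detection or ammo logic.
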(event Input|EnhancedActionEvents|EnhancedInputActionIA_Fire
  (params (ActionValue :type Boolean) (ElapsedSeconds :type Float%20%28double-precision%29) (TriggeredSeconds :type Float%20%28double-precision%29) (InputAction :type Input%20Action%20Object%20Reference :default "/Game/Weapon/IA_Fire.IA_Fire"))
  (:Started
    (CallFunction|StartFire()))
  (:Completed
    (CallFunction|StopFire())))

(fn ConstructionScript)

(fn StartFire()
  (params (NewParam :type BP%20Weapon%20Flame%20Thrower%201%20Object%20Reference))
  (if (not (Variables|Default|GetbActive))
    (Variables|Default|SetbActive true)
    (bind _output_get (Variables|Default|SetAudio_FlameLoop (Variables|Default|GetAudio_FlameLoop)))
    (Audio|Components|Audio|Play _output_get 0.0)
    (bind _output_get_2 (Variables|Default|SetNS_Flame (Variables|Default|GetNS_Flame)))
    (Components|Activation|Activate _output_get_2 false)
    (Audio|Components|Audio|Play (Variables|Default|GetAudio_FlameLoop) 0.0)
    (Development|PrintString "더ㅣ냐?")))

(fn StopFire()
  (if (Variables|Default|GetbActive)
    (Variables|Default|SetbActive false)
    (bind _output_get (Variables|Default|SetAudio_FlameLoop (Variables|Default|GetAudio_FlameLoop)))
    (Audio|Components|Audio|Stop _output_get)
    (bind _output_get_2 (Variables|Default|SetNS_Flame (Variables|Default|GetNS_Flame)))
    (Components|Activation|Deactivate _output_get_2)
    (Development|PrintString "되냐?")))